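; Electric pole prop for the Anime City Suburbs environment that strings four cables to a linked next pole.
; The construction script sets each cable's end to the matching sphere on NextPole, converted into this actor's local space.
; An optional flag randomizes each cable's gravity scale for varied sag, and cables are destroyed when no next pole is valid.
; The ResetWires branch is empty and the event graph holds no logic.
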(event EventBeginPlay)

(event Collision|EventActorBeginOverlap
  (params (OtherActor :type Actor%20Object%20Reference)))

(event EventTick
  (params (DeltaSeconds :type Float%20%28single-precision%29)))

(fn ConstructionScript
  (if (Variables|Default|GetResetWires)
    _
    (else
      _))
  (Utilities|IsValid (Variables|Default|GetNextPole)
    (:Is%20Valid
      (Variables|/Script/CableComponent.CableComponent|SetEndLocation (Variables|Default|GetCable01) (Math|Transform|InverseTransformLocation (Transformation|GetActorTransform) (Transformation|GetWorldLocation (Variables|Default|GetSphere01 (Variables|Default|GetNextPole)))))
      (Variables|/Script/CableComponent.CableComponent|SetEndLocation (Variables|Default|GetCable02) (Math|Transform|InverseTransformLocation (Transformation|GetActorTransform) (Transformation|GetWorldLocation (Variables|Default|GetSphere02 (Variables|Default|GetNextPole)))))
      (Variables|/Script/CableComponent.CableComponent|SetEndLocation (Variables|Default|GetCable03) (Math|Transform|InverseTransformLocation (Transformation|GetActorTransform) (Transformation|GetWorldLocation (Variables|Default|GetSphere03 (Variables|Default|GetNextPole)))))
      (Variables|/Script/CableComponent.CableComponent|SetEndLocation (Variables|Default|GetCable04) (Math|Transform|InverseTransformLocation (Transformation|GetActorTransform) (Transformation|GetWorldLocation (Variables|Default|GetSphere04 (Variables|Default|GetNextPole)))))
      (if (Variables|Default|GetRandomHangingValue)
        (Variables|/Script/CableComponent.CableComponent|SetCableGravityScale (Variables|Default|GetCable01) (Math|Random|RandomFloatinRange 1.0 1e+01))
        (Variables|/Script/CableComponent.CableComponent|SetCableGravityScale (Variables|Default|GetCable02) (Math|Random|RandomFloatinRange 1.0 1e+01))
        (Variables|/Script/CableComponent.CableComponent|SetCableGravityScale (Variables|Default|GetCable03) (Math|Random|RandomFloatinRange 1.0 1e+01))
        (Variables|/Script/CableComponent.CableComponent|SetCableGravityScale (Variables|Default|GetCable04) (Math|Random|RandomFloatinRange 1.0 1e+01))))
    (:Is%20Not%20Valid
      (Components|DestroyComponent (Variables|Default|GetCable01)))))
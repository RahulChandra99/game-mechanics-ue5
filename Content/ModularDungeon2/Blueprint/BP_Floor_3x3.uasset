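; Modular dungeon 3x3 floor tile that assembles its look in the Construction Script from variant settings.
; The AddLowWalls macro adds edge and corner meshes for up to four sides, with cases chaining so each count includes the previous ones.
; FloorType then selects carpet, damage or colored tile materials.
; Grid and Circle types instead destroy the floor mesh, plus the base for Grid, and add a raised replacement mesh.
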(event EventBeginPlay)

(event Collision|EventActorBeginOverlap
  (params (OtherActor :type Actor%20Object%20Reference)))

(event EventTick
  (params (DeltaSeconds :type Float%20%28single-precision%29)))

(fn ConstructionScript
  (bind _returnvalue (Math|Transform|MakeTransform "0.000000,0.000000,90.000000"))
  (bind _floor_3x3 (Variables|Default|GetFloor_3x3))
  (bind _floor_3x3_2 (Variables|Default|GetFloor_3x3))
  (|AddLowWalls
    (:Default
      _)
    (:0
      _)
    (:Floor%20Type
      _))
  (switch Utilities|FlowControl|Switch|SwitchonEN_FloorType (Variables|FloorType|GetFloor%20Type)
    (:NewEnumerator0
      (switch int (Variables|FloorType|GetCarpet)
        (:Default
          (Rendering|Material|SetMaterial _floor_3x3 0 "/Game/ModularDungeon2/Material/MI_ConcreteTiles_Carpet.MI_ConcreteTiles_Carpet" :!label _label))
        (:0
          (goto _label))
        (:1
          (Rendering|Material|SetMaterial _floor_3x3 0 "/Game/ModularDungeon2/Material/MI_ConcreteTiles_CarpetEnd.MI_ConcreteTiles_CarpetEnd"))
        (:2
          (Rendering|Material|SetMaterial _floor_3x3 0 "/Game/ModularDungeon2/Material/MI_ConcreteTiles_CarpetCross.MI_ConcreteTiles_CarpetCross"))))
    (:NewEnumerator1
      (switch int (Variables|FloorType|GetDamage)
        (:Default
          (Rendering|Material|SetMaterial _floor_3x3 0 "/Game/ModularDungeon2/Material/MI_ConcreteTiles_DamageA.MI_ConcreteTiles_DamageA" :!label _label_2))
        (:0
          (goto _label_2))
        (:1
          (Rendering|Material|SetMaterial _floor_3x3 0 "/Game/ModularDungeon2/Material/MI_ConcreteTiles_DamageB.MI_ConcreteTiles_DamageB"))))
    (:NewEnumerator3
      (Rendering|Material|SetMaterial _floor_3x3 0 "/Game/ModularDungeon2/Material/MI_ConcreteTiles_Color.MI_ConcreteTiles_Color"))
    (:NewEnumerator4
      (Components|DestroyComponent _floor_3x3_2)
      (AddComponent|AddStaticMeshComponent false _returnvalue))
    (:NewEnumerator5
      (Components|DestroyComponent _floor_3x3_2)
      (AddComponent|AddStaticMeshComponent false _returnvalue))))
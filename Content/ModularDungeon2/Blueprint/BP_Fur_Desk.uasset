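; BP_Fur_Desk is a modular dungeon furniture prop: a desk with three drawers that can be posed individually.
; The construction script sets each drawer component's relative transform at a fixed X and height, taking its Y offset from the Drawer1, Drawer2 and Drawer3 variables to slide it along that axis.
; The event graph holds only disabled default nodes, so the desk has no runtime behavior.
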(event EventBeginPlay)

(event Collision|EventActorBeginOverlap
  (params (OtherActor :type Actor%20Object%20Reference)))

(event EventTick
  (params (DeltaSeconds :type Float%20%28single-precision%29)))

(fn ConstructionScript
  (Transformation|SetRelativeTransform (Variables|Default|GetFur_Desk_Drawer_1) (Math|Transform|MakeTransform (Math|Vector|MakeVector -63.0 (Math|Conversions|ToFloat(Integer) (Variables|Default|GetDrawer%201)) 75.0)) false false)
  (Transformation|SetRelativeTransform (Variables|Default|GetFur_Desk_Drawer_2) (Math|Transform|MakeTransform (Math|Vector|MakeVector 0.0 (Math|Conversions|ToFloat(Integer) (Variables|Default|GetDrawer%202)) 75.0)) false false)
  (Transformation|SetRelativeTransform (Variables|Default|GetFur_Desk_Drawer_3) (Math|Transform|MakeTransform (Math|Vector|MakeVector 63.0 (Math|Conversions|ToFloat(Integer) (Variables|Default|GetDrawer%203)) 75.0)) false false))